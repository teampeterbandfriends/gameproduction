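; Player character Blueprint handling movement, mouse look, a montage-based Hadouken ability, melee and damage-triggered death.
; Movement includes double jump, crouch and walk toggles, and sprint with timer-driven energy drain and regeneration.
; Tagged-wall overlaps poll WallJump until falling, then lower gravity for a slide that Jump turns into a backward launch.
; Melee input toggles collision on hand components, which the construction script attaches to mesh sockets.
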(event OnComponentBeginOverlap(WallJumpCollision)
  (params (OverlappedComponent :type Primitive%20Component%20Object%20Reference) (OtherActor :type Actor%20Object%20Reference) (OtherComp :type Primitive%20Component%20Object%20Reference) (OtherBodyIndex :type Integer) (bFromSweep :type Boolean) (SweepResult :type Hit%20Result%20Structure%20%28by%20ref%29))
  ;[1 1 1] Jumping
  (if (Actor|ActorHasTag OtherActor "WallJump")
    (Development|PrintString "WALLJUMP!!!!!!!!!!" true true "(R=0.000000,G=0.660000,B=1.000000,A=1.000000)" 5.0)
    (Variables|Default|SetCanWallJump? true :!label _label)
    (bind _returnvalue (CallFunction|WallJump))
    (if (not _returnvalue)
      (Utilities|FlowControl|Delay 0.2)
      (goto _label))))

(event OnComponentEndOverlap(WallJumpCollision)
  (params (OverlappedComponent :type Primitive%20Component%20Object%20Reference) (OtherActor :type Actor%20Object%20Reference) (OtherComp :type Primitive%20Component%20Object%20Reference) (OtherBodyIndex :type Integer))
  ;[1 1 1] Jumping
  (if (Actor|ActorHasTag OtherActor "WallJump")
    (Variables|Default|SetCanWallJump? false)
    (Variables|/Script/Engine.CharacterMovementComponent|SetGravityScale (Variables|Character|GetCharacterMovement) 1.0)
    (Variables|Default|SetCloseToWall? false)))

(event Custom|DecreaseEnergy
  ;[1 1 1] Sprint
  (if (<= (Variables|Attributes|GetMyPlayerEnergy) 0.0)
    (Variables|/Script/Engine.CharacterMovementComponent|SetMaxWalkSpeed (Variables|Character|GetCharacterMovement) 4e+02)
    (Utilities|Time|ClearandInvalidateTimerbyHandle (stale Input|ActionEvents|InputActionSprint _returnvalue))
    (bind _returnvalue (Utilities|Time|SetTimerbyEvent (delegate Custom|IncreaseEnergy) 0.05 true))
    (else
      (Variables|Attributes|SetMyPlayerEnergy (- (Variables|Attributes|GetMyPlayerEnergy) 1.0)))))

(event Custom|IncreaseEnergy
  ;[1 1 1] Sprint
  (if (not (>= (Variables|Attributes|GetMyPlayerEnergy) (Variables|Attributes|GetMyPlayerMaxEnergy)))
    (Variables|Attributes|SetMyPlayerEnergy (+ (Variables|Attributes|GetMyPlayerEnergy) (Variables|Attributes|GetMyPlayerEnergyRegen)))
    (Utilities|Time|ClearandInvalidateTimerbyHandle (stale Input|ActionEvents|InputActionSprint _returnvalue_2))
    (Utilities|Time|ClearandInvalidateTimerbyHandle (stale Custom|DecreaseEnergy _returnvalue))))

(event EventBeginPlay)

(event Collision|EventActorBeginOverlap
  (params (OtherActor :type Actor%20Object%20Reference)))

(event EventOnLanded
  (params (Hit :type Hit%20Result%20Structure%20%28by%20ref%29))
  ;[1 1 1] Jumping
  ;;[1 1 1] Landing
  (Variables|Default|SetJumpCounter 0)
  (Variables|Default|SetInAir? false)
  (Variables|Default|SetDoubleJump false)
  (Variables|Default|SetCanCast? true)
  (Variables|Default|SetCloseToWall? false))

(event EventTick
  (params (DeltaSeconds :type Float%20%28single-precision%29))
  (if (Math|Vector|NotEqual(Vector) (Transformation|GetComponentVelocity (Variables|Collision|GetCapsuleComponent)) "0, 0, 0" 0.0)
    (Animation|StopAnimMontage "/Game/_MyContent/Assets/Animations/Mon_Hadouken.Mon_Hadouken")
    (Variables|Default|SetIsCasting? false)))

(event Game|Damage|EventAnyDamage
  (params (Damage :type Float%20%28single-precision%29) (DamageType :type Damage%20Type%20Object%20Reference) (InstigatedBy :type Controller%20Object%20Reference) (DamageCauser :type Actor%20Object%20Reference))
  (bind _output_get (Variables|Attributes|SetMyPlayerHealth (- Damage (Variables|Attributes|GetMyPlayerHealth))))
  (if (<= _output_get 0.0)
    (Default|CallPlayerDied)))

(event Input|ActionEvents|InputActionJump
  (params (Key :type Key%20Structure))
  (bind _returnvalue (Transformation|GetActorForwardVector))
  (bind _returnvalue_2 (* (Math|Vector|MakeVector (.x _returnvalue) (.y _returnvalue) 0.0) -2e+02))
  ;[1 1 1] Jumping
  (:Pressed
    (if (Variables|Default|GetCloseToWall?)
      (Pawn|Input|AddControllerYawInput 3.6e+02)
      (Character|LaunchCharacter (Math|Vector|MakeVector (.x _returnvalue_2) (.y _returnvalue_2) 4e+02) false false)
      (Variables|/Script/Engine.CharacterMovementComponent|SetGravityScale (Variables|Character|GetCharacterMovement) 1.0)
      (else
        (if (Variables|Default|GetIsCasting?)
          (Animation|StopAnimMontage "/Game/_MyContent/Assets/Animations/Mon_Hadouken.Mon_Hadouken"))
        (if (< (Variables|Default|GetJumpCounter) (Variables|Default|GetJumpMaxCount))
          (bind _output_get (Variables|Default|SetJumpCounter (+ (Variables|Default|GetJumpCounter) 1)))
          (if (>= _output_get 2)
            (Character|Jump)
            (Variables|Default|SetInAir? true)
            (Variables|Default|SetDoubleJump true)
            (Utilities|FlowControl|Delay 0.2)
            (Variables|Default|SetDoubleJump false)
            (else
              (Character|Jump)
              (Variables|Default|SetInAir? true)))))))
  (:Released
    (Character|StopJumping)))

(event Input|ActionEvents|InputActionAbility1
  (params (Key :type Key%20Structure))
  ;[1 1 1] Casting Ability 1
  (:Pressed
    (if (not (Variables|Default|GetInAir?))
      (if (Variables|Default|GetCanCast?)
        (Development|PrintString "Hadouken")
        (Animation|Montage|MontagePlay (Components|SkeletalMesh|GetAnimInstance (Variables|Character|GetMesh)) "/Game/_MyContent/Assets/Animations/Mon_Hadouken.Mon_Hadouken" 1.0 "MontageLength" 0.0 true)
        (Variables|Default|SetCanCast? false)
        (Variables|Default|SetIsCasting? true)
        (Utilities|FlowControl|Delay 3.0)
        (Variables|Default|SetCanCast? true)
        (Variables|Default|SetIsCasting? false)))))

(event Input|ActionEvents|InputActionSprint
  (params (Key :type Key%20Structure))
  (bind _charactermovement (Variables|Character|GetCharacterMovement))
  ;[1 1 1] Sprint
  (:Pressed
    (Variables|/Script/Engine.CharacterMovementComponent|SetMaxWalkSpeed _charactermovement 6e+02)
    (bind _returnvalue (Utilities|Time|SetTimerbyEvent (delegate Custom|DecreaseEnergy) 0.05 true))
    (Utilities|Time|ClearandInvalidateTimerbyHandle (stale _returnvalue_2))
    (Utilities|Time|ClearandInvalidateTimerbyHandle (stale Custom|DecreaseEnergy _returnvalue)))
  (:Released
    (Variables|/Script/Engine.CharacterMovementComponent|SetMaxWalkSpeed _charactermovement 3.5e+02)
    (bind _returnvalue_2 (Utilities|Time|SetTimerbyEvent (delegate Custom|IncreaseEnergy) 0.05 true))
    (Utilities|Time|ClearandInvalidateTimerbyHandle _returnvalue)))

(event Input|ActionEvents|InputActionWalk
  (params (Key :type Key%20Structure))
  (bind _charactermovement (Variables|Character|GetCharacterMovement))
  ;[1 1 1] Walk
  (:Pressed
    (if (Variables|Default|GetIsWalking?)
      (Variables|/Script/Engine.CharacterMovementComponent|SetMaxWalkSpeed _charactermovement 3.5e+02)
      (Variables|Default|SetIsWalking? false)
      (else
        (Variables|/Script/Engine.CharacterMovementComponent|SetMaxWalkSpeed _charactermovement 5e+01)
        (Variables|Default|SetIsWalking? true)))))

(event Input|ActionEvents|InputActionCrouch
  (params (Key :type Key%20Structure))
  ;[1 1 1] Crouch
  (:Pressed
    (if (AI|Components|NavMovement|IsCrouching (Variables|Character|GetCharacterMovement))
      (Character|UnCrouch)
      (else
        (Character|Crouch)))))

(event Input|ActionEvents|InputActionMeleeAttack
  (params (Key :type Key%20Structure))
  ;[1 1 1] Melee Attack
  (:Pressed
    (Variables|Default|SetIsPunching? true)
    (Collision|SetCollisionEnabled (Variables|Default|GetRightHandCollision) "QueryAndPhysics"))
  (:Released
    (Variables|Default|SetIsPunching? false)
    (Collision|SetCollisionEnabled (Variables|Default|GetLeftHandCollision) "NoCollision")))

(event Input|AxisEvents|InputAxisMoveRight
  (params (AxisValue :type Float%20%28single-precision%29))
  ;[1 1 1] Basic Player Movement Input (Keyboard)
  (Pawn|Input|AddMovementInput (Math|Vector|GetRightVector (Math|Rotator|MakeRotator 0.0 0.0 (.Yaw (Math|Rotator|BreakRotator (Pawn|GetControlRotation :!class /Script/Engine.Pawn))))) AxisValue false))

(event Input|AxisEvents|InputAxisMoveForward
  (params (AxisValue :type Float%20%28single-precision%29))
  ;[1 1 1] Basic Player Movement Input (Keyboard)
  (Pawn|Input|AddMovementInput (Math|Vector|GetForwardVector (Math|Rotator|MakeRotator 0.0 0.0 (.Yaw (Math|Rotator|BreakRotator (Pawn|GetControlRotation :!class /Script/Engine.Pawn))))) AxisValue false))

(event Input|AxisEvents|InputAxisTurn
  (params (AxisValue :type Float%20%28single-precision%29))
  ;[1 1 1] Player Looking Around (Mouse)
  (Pawn|Input|AddControllerYawInput AxisValue))

(event Input|AxisEvents|InputAxisLookUp
  (params (AxisValue :type Float%20%28single-precision%29))
  ;[1 1 1] Player Looking Around (Mouse)
  (Pawn|Input|AddControllerPitchInput AxisValue))

(fn ConstructionScript
  (bind _mesh (Variables|Character|GetMesh))
  (Transformation|AttachComponentToComponent (Variables|Default|GetLeftHandCollision) _mesh "middle_01_l" "SnapToTarget" "KeepRelative" "KeepWorld" true)
  (Transformation|AttachComponentToComponent (Variables|Default|GetRightHandCollision) _mesh "middle_01_r" "SnapToTarget" "KeepRelative" "KeepWorld" true))

(fn WallJump
  (bind _returnvalue (Transformation|GetVelocity))
  (bind _returnvalue_2 (< (.z _returnvalue) 0.0))
  (if _returnvalue_2
    (Variables|/Script/Engine.CharacterMovementComponent|SetGravityScale (Variables|Character|GetCharacterMovement) 0.3)
    (bind _output_get (Variables|Default|SetCloseToWall? true))
    (return _output_get)
    (else
      (return _returnvalue_2))))