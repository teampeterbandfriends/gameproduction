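; Game manager Blueprint that owns the UI widgets and the current game state.
; Init creates the store, HUD, main menu, pause and quit widgets, initializes the player, then enters Running.
; SetState hides all UI on a change, shows that state's widget and toggles the mouse cursor; Pause has no state branch.
; ResetGame is unfinished: it finds ThirdPersonCharacter actors, but its relocation node is unconnected.
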(event EventBeginPlay)

(event Collision|EventActorBeginOverlap
  (params (OtherActor :type Actor%20Object%20Reference)))

(event EventTick
  (params (DeltaSeconds :type Float%20%28single-precision%29)))

(fn ConstructionScript)

(fn Init
  (CallFunction|CreateUI)
  (Default|Init (Variables|Default|GetMy%20Player))
  (CallFunction|ResetGame)
  (CallFunction|SetState "NewEnumerator0"))

(fn CreateUI
  (bind _returnvalue (UserInterface|CreateWidget "/Game/_MyContent/UI/Widget_Store-Vendor.Widget_Store-Vendor_C"))
  (bind _output_get (Variables|Default|SetWidget_Store _returnvalue))
  (UserInterface|Viewport|AddtoViewport _output_get 0)
  (bind _returnvalue_2 (UserInterface|CreateWidget "/Game/_MyContent/UI/Widget_HUD.Widget_HUD_C"))
  (bind _output_get_2 (Variables|Default|SetWidget_HUD _returnvalue_2))
  (UserInterface|Viewport|AddtoViewport _output_get_2 0)
  (bind _returnvalue_3 (UserInterface|CreateWidget "/Game/_MyContent/UI/Widget_MainMenu.Widget_MainMenu_C"))
  (bind _output_get_3 (Variables|Default|SetMain%20Menu _returnvalue_3))
  (UserInterface|Viewport|AddtoViewport _output_get_3 0)
  (bind _returnvalue_4 (UserInterface|CreateWidget "/Game/_MyContent/UI/Widget_Pause.Widget_Pause_C"))
  (bind _output_get_4 (Variables|Default|SetPause _returnvalue_4))
  (UserInterface|Viewport|AddtoViewport _output_get_4 0)
  (bind _returnvalue_5 (UserInterface|CreateWidget "/Game/_MyContent/UI/Widget_Quit.Widget_Quit_C"))
  (bind _output_get_5 (Variables|Default|SetQuit _returnvalue_5))
  (UserInterface|Viewport|AddtoViewport _output_get_5 0))

(fn SetState
  (params (New%20State :type _GameStates%20Enum :default "NewEnumerator0"))
  (if (Utilities|Enum|NotEqual(Enum) New%20State (Variables|Default|GetCurrent%20Game%20State))
    (CallFunction|HideUI)
    (bind _output_get (Variables|Default|SetCurrent%20Game%20State New%20State))
    (switch Utilities|FlowControl|Switch|Switchon_GameStates _output_get
      (:NewEnumerator0
        (Widget|SetVisibility (Variables|Default|GetWidget_HUD) "Visible")
        (CallFunction|ShowMouse false))
      (:NewEnumerator3
        (Widget|SetVisibility (Variables|Default|GetQuit) "Visible")
        (CallFunction|ShowMouse true :!label _label))
      (:NewEnumerator5
        (Widget|SetVisibility (Variables|Default|GetWidget_Store) "Visible")
        (goto _label))
      (:NewEnumerator6
        (Widget|SetVisibility (Variables|Default|GetMain%20Menu) "Visible")
        (goto _label)))))

(fn GetState
  (return (Variables|Default|GetCurrent%20Game%20State)))

(fn ShowHUD
  (params (Visible :type Boolean))
  (bind _widget_hud (Variables|Default|GetWidget_HUD))
  (if Visible
    (Widget|SetVisibility _widget_hud "Visible")
    (else
      (Widget|SetVisibility _widget_hud "Hidden"))))

(fn ResetGame
  (bind _outactors (Actor|GetAllActorsOfClass "/Game/ThirdPersonBP/Blueprints/ThirdPersonCharacter.ThirdPersonCharacter_C")))