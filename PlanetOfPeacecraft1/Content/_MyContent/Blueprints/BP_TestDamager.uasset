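; BP_TestDamager is a damage volume that drains a BP_MyPlayer's health while it is inside the Box.
; Box overlaps store the player and toggle InsideVolume, which lets Tick run ContinueDamage to apply DamageRate scaled by delta time until AccumDamage reaches MaxDamage.
; AccumDamage is never reset on exit, so the cap spans repeated entries.
; StartDamage defines a clamped instant hit but is not called in this Blueprint.
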(event OnComponentBeginOverlap(Box)
  (params (OverlappedComponent :type Primitive%20Component%20Object%20Reference) (OtherActor :type Actor%20Object%20Reference) (OtherComp :type Primitive%20Component%20Object%20Reference) (OtherBodyIndex :type Integer) (bFromSweep :type Boolean) (SweepResult :type Hit%20Result%20Structure%20%28by%20ref%29))
  (bind _asbp_my_player (Utilities|Casting|CastToBP_MyPlayer OtherActor))
  (Variables|Default|SetInsideVolume true)
  (Variables|Default|SetMyPlayer _asbp_my_player))

(event OnComponentEndOverlap(Box)
  (params (OverlappedComponent :type Primitive%20Component%20Object%20Reference) (OtherActor :type Actor%20Object%20Reference) (OtherComp :type Primitive%20Component%20Object%20Reference) (OtherBodyIndex :type Integer))
  (Utilities|Casting|CastToBP_MyPlayer OtherActor)
  (Variables|Default|SetInsideVolume false))

(event EventBeginPlay)

(event Collision|EventActorBeginOverlap
  (params (OtherActor :type Actor%20Object%20Reference)))

(event EventTick
  (params (DeltaSeconds :type Float%20%28single-precision%29))
  (if (Variables|Default|GetInsideVolume)
    (CallFunction|ContinueDamage)))

(fn ConstructionScript)

(fn StartDamage
  (bind _output_get (Variables|Default|SetAccumDamage (Variables|Default|GetInstantDamage))) ; Apply INstant Damage
  (if (> _output_get (Variables|Default|GetMaxDamage)) ; Clamping accumulative damage to maximum damage
    (Variables|Default|SetAccumDamage (Variables|Default|GetMaxDamage)))
  (Default|ChangeHealth (Variables|Default|GetMyPlayer) (* (Variables|Default|GetAccumDamage) -1.0)))

(fn ContinueDamage
  (bind _returnvalue (Utilities|Time|GetWorldDeltaSeconds))
  (bind _damagerate (Variables|Default|GetDamageRate))
  (bind _returnvalue_2 (* _damagerate _returnvalue))
  (if (< (Variables|Default|GetAccumDamage) (Variables|Default|GetMaxDamage)) ; Is accumulative damage less than maximum?
    (Variables|Default|SetAccumDamage (+ _returnvalue_2 (Variables|Default|GetAccumDamage)))
    (Default|ChangeHealth (Variables|Default|GetMyPlayer) (* _returnvalue_2 -1.0))))