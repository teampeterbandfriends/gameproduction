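; BP_Lightning is a lightning spell actor that instantly kills enemies it touches and pays out currency.
; On capsule overlap, a Sequence tests the other actor against AICharacter, AIBulkierEnemy and AIBoss, destroys it, and adds a tier-based reward to the GameManager's Currency.
; The bulkier enemy and boss branches also destroy the lightning, while the AICharacter branch leaves it alive.
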(event OnComponentBeginOverlap(Capsule)
  (params (OverlappedComponent :type Primitive%20Component%20Object%20Reference) (OtherActor :type Actor%20Object%20Reference) (OtherComp :type Primitive%20Component%20Object%20Reference) (OtherBodyIndex :type Integer) (bFromSweep :type Boolean) (SweepResult :type Hit%20Result%20Structure%20%28by%20ref%29))
  (Utilities|FlowControl|Sequence
    (:then_0
      (bind _asaicharacter (Utilities|Casting|CastToAICharacter OtherActor))
      (Actor|DestroyActor _asaicharacter)
      (bind _game_manager (CallFunction|GetGameManager))
      (Variables|/Game/_MyContent/Blueprints/_GameManager._GameManager_C|SetCurrency _game_manager (+ (Variables|/Game/_MyContent/Blueprints/_GameManager._GameManager_C|GetCurrency _game_manager) 2e+02)))
    (:then_1
      (bind _asaibulkier_enemy (Utilities|Casting|CastToAIBulkierEnemy OtherActor))
      (Actor|DestroyActor _asaibulkier_enemy)
      (bind _game_manager_2 (CallFunction|GetGameManager))
      (Variables|/Game/_MyContent/Blueprints/_GameManager._GameManager_C|SetCurrency _game_manager_2 (+ (Variables|/Game/_MyContent/Blueprints/_GameManager._GameManager_C|GetCurrency _game_manager_2) 5e+02))
      (Actor|DestroyActor))
    (:then_2
      (bind _asaiboss (Utilities|Casting|CastToAIBoss OtherActor))
      (Actor|DestroyActor _asaiboss)
      (bind _game_manager_3 (CallFunction|GetGameManager))
      (Variables|/Game/_MyContent/Blueprints/_GameManager._GameManager_C|SetCurrency _game_manager_3 (+ (Variables|/Game/_MyContent/Blueprints/_GameManager._GameManager_C|GetCurrency _game_manager_3) 1e+03))
      (Actor|DestroyActor))))

(event EventBeginPlay)

(event Collision|EventActorBeginOverlap
  (params (OtherActor :type Actor%20Object%20Reference)))

(event EventTick
  (params (DeltaSeconds :type Float%20%28single-precision%29)))

(fn ConstructionScript)