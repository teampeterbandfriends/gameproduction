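; BP_FireSpell is a fire spell projectile that kills AI characters and rewards the player with currency.
; On BeginPlay it sets a short lifespan and moves forward without sweep in a repeating Delay loop instead of Tick.
; When its Damager component overlaps an AICharacter, it destroys that character, adds currency to the GameManager, destroys itself and prints the new total.
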(event OnComponentBeginOverlap(Damager)
  (params (OverlappedComponent :type Primitive%20Component%20Object%20Reference) (OtherActor :type Actor%20Object%20Reference) (OtherComp :type Primitive%20Component%20Object%20Reference) (OtherBodyIndex :type Integer) (bFromSweep :type Boolean) (SweepResult :type Hit%20Result%20Structure%20%28by%20ref%29))
  (bind _asaicharacter (Utilities|Casting|CastToAICharacter OtherActor))
  (Actor|DestroyActor _asaicharacter)
  (bind _game_manager (CallFunction|GetGameManager))
  (bind _output_get (Variables|/Game/_MyContent/Blueprints/_GameManager._GameManager_C|SetCurrency _game_manager (+ (Variables|/Game/_MyContent/Blueprints/_GameManager._GameManager_C|GetCurrency _game_manager) 5e+02)))
  (Actor|DestroyActor)
  (Development|PrintString (Utilities|String|ToString(Float) _output_get)))

(event EventBeginPlay
  (Actor|SetLifeSpan 3.0)
  (Transformation|AddActorWorldOffset (* (Transformation|GetActorForwardVector) 2e+01) :!label _label)
  (Utilities|FlowControl|Delay 0.01)
  (goto _label))

(event Collision|EventActorBeginOverlap
  (params (OtherActor :type Actor%20Object%20Reference)))

(event EventTick
  (params (DeltaSeconds :type Float%20%28single-precision%29)))

(fn ConstructionScript)