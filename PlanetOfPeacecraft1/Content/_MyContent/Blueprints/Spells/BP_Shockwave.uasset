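; Shockwave spell actor that expands as a ring, killing AI characters it touches, and removes itself after a brief lifetime.
; A fast looping timer grows OuterRing exponentially in X and Y, adding the same absolute scale increment to InnerRing to keep their difference constant.
; OuterRing overlaps destroy any AICharacter, award currency through the game manager and print the new total.
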(event OnComponentBeginOverlap(OuterRing)
  (params (OverlappedComponent :type Primitive%20Component%20Object%20Reference) (OtherActor :type Actor%20Object%20Reference) (OtherComp :type Primitive%20Component%20Object%20Reference) (OtherBodyIndex :type Integer) (bFromSweep :type Boolean) (SweepResult :type Hit%20Result%20Structure%20%28by%20ref%29))
  (bind _asaicharacter (Utilities|Casting|CastToAICharacter OtherActor))
  (Actor|DestroyActor _asaicharacter)
  (bind _game_manager (CallFunction|GetGameManager))
  (bind _output_get (Variables|/Game/_MyContent/Blueprints/_GameManager._GameManager_C|SetCurrency _game_manager (+ (Variables|/Game/_MyContent/Blueprints/_GameManager._GameManager_C|GetCurrency _game_manager) 5e+02)))
  (Development|PrintString (Utilities|String|ToString(Float) _output_get)))

(event Custom|Shockwave
  (bind _innerring (Variables|Default|GetInnerRing))
  (bind _outerring (Variables|Default|GetOuterRing))
  (bind _returnvalue (Transformation|GetWorldScale _outerring))
  (bind _returnvalue_2 (Transformation|GetWorldScale _innerring))
  (bind _returnvalue_3 (* _returnvalue 1.05))
  (bind (_x _y _z) (Math|Vector|BreakVector _returnvalue))
  (bind (_x_2 _y_2 _z_2) (Math|Vector|BreakVector _returnvalue_2))
  (bind _x_3 (Math|Vector|BreakVector _returnvalue_3))
  (bind _returnvalue_4 (- _x_3 _x))
  (bind _returnvalue_5 (+ _x_2 _returnvalue_4))
  (Transformation|SetWorldScale3D _innerring (Math|Vector|MakeVector _returnvalue_5 _returnvalue_5 _z_2))
  (Transformation|SetWorldScale3D _outerring (Math|Vector|MakeVector _x_3 _x_3 _z)))

(event EventBeginPlay
  (Utilities|Time|SetTimerbyEvent (delegate Custom|Shockwave) 0.01 true)
  (Utilities|FlowControl|Delay 0.3)
  (Actor|DestroyActor))

(event Collision|EventActorBeginOverlap
  (params (OtherActor :type Actor%20Object%20Reference)))

(event EventTick
  (params (DeltaSeconds :type Float%20%28single-precision%29)))

(fn ConstructionScript)